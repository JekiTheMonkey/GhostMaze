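; AI controller for bots that runs an assigned behavior tree and seeds a patrol destination.
; On BeginPlay it starts the tree if valid, then calls RandomNewDestination.
; That function picks a random reachable navigation point within PatrolRadius of the controlled pawn and writes it to the Destination blackboard key, printing an error if none is found.
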(event `self.ReceiveBeginPlay`
  (bind _behaviortree (`self.BehaviorTree`))
  (`|ExecutionSequence`
    (:`then_0`
      (`/Engine/EditorBlueprintResources/StandardMacros.IsValid` _behaviortree
        (:`Is Valid`
          (`self.RunBehaviorTree` _behaviortree))))
    (:`then_1`
      (`self.RandomNewDestination`))))

(fn `RandomNewDestination`
  (bind _returnvalue (`self.K2_GetPawn`))
  (bind _blackboard (`self.Blackboard`))
  (bind (_randomlocation _returnvalue_2) (`NavigationSystemV1.K2_GetRandomReachablePointInRadius` (`self.K2_GetActorLocation` _returnvalue) (`self.PatrolRadius`) null null))
  (`/Engine/EditorBlueprintResources/StandardMacros.IsValid` _returnvalue
    (:`Is Valid`
      (`/Engine/EditorBlueprintResources/StandardMacros.IsValid` _blackboard
        (:`Is Valid`
          (if _returnvalue_2
            (`BlackboardComponent.SetValueAsVector` _blackboard "Destination" _randomlocation)
            (else
              (`KismetSystemLibrary.PrintString` "Failed to get a random destination in radius" true true (struct :`R` 1.0 :`A` 1.0)))))))))

(fn `UserConstructionScript`)